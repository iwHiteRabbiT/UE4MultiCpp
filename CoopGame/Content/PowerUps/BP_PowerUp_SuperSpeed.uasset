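; Super speed power-up that doubles the activating actor's walking speed while active.
; On state change, it scales MaxWalkSpeed on the target's CharacterMovementComponent by two, then divides by two when deactivated, provided RActivatedTargetActor is valid.
; It then calls the parent state-change handler; the change is relative to the current speed rather than restoring a stored original value.
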(event `self.OnPowerUpStateChange`
  (params (bIsActive :type Boolean))
  (bind _r_activatedtargetactor (`self.R_ActivatedTargetActor`))
  (bind _returnvalue (`self.GetComponentByClass` _r_activatedtargetactor "/Script/Engine.CharacterMovementComponent"))
  (`|ExecutionSequence`
    (:`then_0`
      (`/Engine/EditorBlueprintResources/StandardMacros.IsValid` _r_activatedtargetactor
        (:`Is Valid`
          (if bIsActive
            (set `CharacterMovementComponent.MaxWalkSpeed` (* (`CharacterMovementComponent.MaxWalkSpeed` _returnvalue) 2.0) _returnvalue)
            (else
              (set `CharacterMovementComponent.MaxWalkSpeed` (/ (`CharacterMovementComponent.MaxWalkSpeed` _returnvalue) 2.0) _returnvalue))))))
    (:`then_1`
      (`parent.OnPowerUpStateChange` bIsActive))))

(fn `UserConstructionScript`)