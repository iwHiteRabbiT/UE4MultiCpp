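; Behavior tree service that picks the nearest hostile target for an AI pawn and writes it to the blackboard.
; Each tick it scans actors known through sight perception, keeping those with health above zero that are not friendly to the pawn.
; The closest by straight-line distance becomes the best target; the key is set to None when no actor qualifies.
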(event `self.ReceiveTickAI`
  (params (OwnerController :type "AIController Object Reference") (ControlledPawn :type "Pawn Object Reference") (DeltaSeconds :type "Float (single-precision)"))
  (set `self.BestTargetActor` null)
  (set `self.NearestTargetDist` 100000000.0)
  (for _array_element (`AIPerceptionComponent.GetKnownPerceivedActors` (`Actor.GetComponentByClass` ControlledPawn "/Script/AIModule.AIPerceptionComponent") "/Script/AIModule.AISense_Sight")
    (if (> (`SHealthComponent.R_Health` (`Actor.GetComponentByClass` _array_element "/Script/CoopGame.SHealthComponent")) 0.0)
      (if (not (`SHealthComponent.IsFriendly` _array_element ControlledPawn))
        (bind _returnvalue (`KismetMathLibrary.VSize` (- (`Actor.K2_GetActorLocation` _array_element) (`Actor.K2_GetActorLocation` ControlledPawn))))
        (if (< _returnvalue (`self.NearestTargetDist`))
          (set `self.NearestTargetDist` _returnvalue)
          (set `self.BestTargetActor` _array_element)))))
  (`BTFunctionLibrary.SetBlackboardValueAsObject` (`self.BBBestTargetActor`) (`self.BestTargetActor`)))